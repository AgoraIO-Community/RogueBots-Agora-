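; Game mode Blueprint that switches between the screens of a video call app: introduction, video settings, device test and video call.
; Each view function calls RemoveAllWidgets, then adds its stored widget to the viewport, so one screen shows at a time.
; A further function forwards button text to the introduction widget's video settings button.
; BeginPlay, Tick and the construction script are empty, and widget creation happens outside these graphs.
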(event `self.ReceiveBeginPlay`)

(event `self.ReceiveTick`
  (params (DeltaSeconds :type "Float (single-precision)")))

(fn `SetDeviceTestView`
  (`WidgetLayoutLibrary.RemoveAllWidgets`)
  (`UserWidget.AddToViewport` (`self.DeviceTestWidget_BP`) 0))

(fn `SetIntroductionView`
  (`WidgetLayoutLibrary.RemoveAllWidgets`)
  (`UserWidget.AddToViewport` (`self.IntroductionWidget_BP`) 0))

(fn `SetVideoCallView`
  (`WidgetLayoutLibrary.RemoveAllWidgets`)
  (`UserWidget.AddToViewport` (`self.VideoCallWidget_BP`) 0))

(fn `SetVideoSettingsButtonText`
  (params (Text :type String))
  (`/Game/Widgets_BP/IntroductionWidget_BP.SetVideoSettingsButtonText` (`self.IntroductionWidget_BP`) Text))

(fn `SetVideoSettingsView`
  (`WidgetLayoutLibrary.RemoveAllWidgets`)
  (`UserWidget.AddToViewport` (`self.VideoSettintsWidget_BP`) 0))

(fn `UserConstructionScript`)